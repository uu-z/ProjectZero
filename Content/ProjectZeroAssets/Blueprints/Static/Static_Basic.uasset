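; Static_Basic is a data-driven static world actor that loads its info and current state from a table row on construction.
; Lifecycle and sphere overlaps with InteractionComponent owners trigger keyed lookups that swap the mesh, resize the sphere, play sounds or run actions like self-destruction.
; Overlaps also write a state bool map, which Tick syncs and broadcasts as changes, letting Effect tasks spawn row-defined actors.
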(event `Event Bind`
  (`|ExecutionSequence`
    (:`then_0`
      (add `self.UpdateBool` (delegate `UpdateBool_Event`)))
    (:`then_1`
      (add `self.OnDestroyed` (delegate `OnDestroyed_Event_0`)))))

(event `self.ReceiveBeginPlay`
  (`self.Event Bind`)
  (`self.Event Trigger` "NewEnumerator3"))

(event `UpdateBool_Event` :!signature `self.UpdateBool`
  (params (Key :type "/Game/ProjectZeroCore/StaticSys/E_StaticBool Enum") (Value :type Boolean))
  (bind (_boolmap _tasks _effects) (break `/Game/ProjectZeroCore/StaticSys/S_StaticState` (`self.StateSync`)))
  (switch `/Game/ProjectZeroCore/StaticSys/E_StaticBool` Key
    (:`NewEnumerator1`
      (for _array_element _tasks
        (switch `/Game/ProjectZeroCore/StaticSys/E_StaticTask` _array_element
          (:`NewEnumerator1`
            ;[0.479 0.4912 1] Effect
            (`/Game/ProjectZeroCore/Utils/ActorMacros.CompareBoolExec` Value true
              (:`true`
                (for _array_element_2 _effects
                  (bind _out_row (`/Game/ProjectZeroCore/Utils/ObjMacros.GetRow` _array_element_2))
                  (`|SpawnActorFromClass` (`.Class_93_1EE3FCBBE446E2152661DBA9E3660676` (break `/Game/ProjectZeroCore/EffectSys/S_Effect1` _out_row)) (`self.GetTransform`) "Undefined" "OverrideRootScale" null _out_row))))))))))

(event `self.SphereCollision.OnComponentBeginOverlap`
  (params (OverlappedComponent :type "PrimitiveComponent Object Reference") (OtherActor :type "Actor Object Reference") (OtherComp :type "PrimitiveComponent Object Reference") (OtherBodyIndex :type Integer) (bFromSweep :type Boolean) (SweepResult :type "HitResult Structure (by ref)"))
  (`/Engine/EditorBlueprintResources/StandardMacros.IsValid` (`self.GetComponentByClass` OtherActor "/Game/ProjectZeroAssets/Blueprints/Components/Interaction/InteractionComponent.InteractionComponent_C")
    (:`Is Valid`
      (`BlueprintMapLibrary.Map_Add` (`.BoolMap_4_6E1DD9AF4345D628040E4F9E91B2D094` (break `/Game/ProjectZeroCore/StaticSys/S_StaticState` (`self.StateSync`))) "NewEnumerator1" true)
      (`self.Event Trigger` "NewEnumerator1"))))

(event `OnDestroyed_Event_0` :!signature `self.OnDestroyed`
  (params (DestroyedActor :type "Actor Object Reference"))
  (`self.Event Trigger` "NewEnumerator4"))

(event `self.SphereCollision.OnComponentEndOverlap`
  (params (OverlappedComponent :type "PrimitiveComponent Object Reference") (OtherActor :type "Actor Object Reference") (OtherComp :type "PrimitiveComponent Object Reference") (OtherBodyIndex :type Integer))
  (`/Engine/EditorBlueprintResources/StandardMacros.IsValid` (`self.GetComponentByClass` OtherActor "/Game/ProjectZeroAssets/Blueprints/Components/Interaction/InteractionComponent.InteractionComponent_C")
    (:`Is Valid`
      (`BlueprintMapLibrary.Map_Add` (`.BoolMap_4_6E1DD9AF4345D628040E4F9E91B2D094` (break `/Game/ProjectZeroCore/StaticSys/S_StaticState` (`self.StateSync`))) "NewEnumerator1")
      (`self.Event Trigger` "NewEnumerator2"))))

(event `self.ReceiveTick`
  (params (DeltaSeconds :type "Float (single-precision)"))
  ;[1 0.3622 0.187] Tick
  (`|ExecutionSequence`
    (:`then_0`
      (bind (_key _value) (`/Game/ProjectZeroCore/Utils/ObjMacros.SyncBoolMap` (`.BoolMap_4_6E1DD9AF4345D628040E4F9E91B2D094` (break `/Game/ProjectZeroCore/StaticSys/S_StaticState` (`self.StateSync`))) (`.BoolMap_4_6E1DD9AF4345D628040E4F9E91B2D094` (break `/Game/ProjectZeroCore/StaticSys/S_StaticState` (`.__State_22_50B4A14FC94F79B01422AFB3C06B3710` (break `/Game/ProjectZeroCore/StaticSys/S_Static` (`self.Info`))))))
        (:`Then`
          (`self.UpdateBool` (cast `/Game/ProjectZeroCore/StaticSys/E_StaticBool` _key) _value))))))

(event `Event Trigger`
  (params (Key :type "/Game/ProjectZeroCore/StaticSys/E_StaticUpdateType Enum"))
  (bind (_row _class _curstate _statemap ___state _meshmap _soundmap _actionmap) (break `/Game/ProjectZeroCore/StaticSys/S_Static` (`self.Info`)))
  (bind (_value _returnvalue) (`BlueprintMapLibrary.Map_Find` _meshmap Key))
  (bind (_value_2 _returnvalue_2) (`BlueprintMapLibrary.Map_Find` _soundmap Key))
  (bind (_value_3 _returnvalue_3) (`BlueprintMapLibrary.Map_Find` _actionmap Key))
  ;[0.3671 1 0.8463] Event Trigger
  (`|ExecutionSequence`
    (:`then_0`
      (if _returnvalue
        (`StaticMeshComponent.SetStaticMesh` (`self.StaticMesh`) _value)
        (`SphereComponent.SetSphereRadius` (`self.SphereCollision`) (* (`.SphereRadius` (`KismetMathLibrary.BreakBoxSphereBounds` (`StaticMesh.GetBounds` _value))) 2.0) true)))
    (:`then_1`
      (if _returnvalue_2
        (`GameplayStatics.PlaySoundAtLocation` _value_2)))
    (:`then_2`
      (if _returnvalue_3
        (switch `/Game/ProjectZeroCore/StaticSys/E_StaticAction` _value_3
          (:`NewEnumerator1`
            (`self.K2_DestroyActor`))
          (:`NewEnumerator2`
            (`KismetSystemLibrary.PrintString` "Test")))))))

(fn `UserConstructionScript`
  (bind _out_row (`/Game/ProjectZeroCore/Utils/ObjMacros.GetRow` (`.Row_2_8CCA2E30454E3D0F1C291A9AA0C067FA` (break `/Game/ProjectZeroCore/StaticSys/S_Static` (`self.Info`)))))
  (bind _output_get (set `self.Info` _out_row))
  (`|ExecutionSequence`
    (:`then_0`
      (bind (_row _class _curstate _statemap) (break `/Game/ProjectZeroCore/StaticSys/S_Static` _output_get))
      (bind _output_get_2 (set `self.StateMap` _statemap))
      (bind _output_get_3 (set `self.CurState` _curstate))
      (set `self.StateSync` (`BlueprintMapLibrary.Map_Find` _output_get_2 _output_get_3)))))