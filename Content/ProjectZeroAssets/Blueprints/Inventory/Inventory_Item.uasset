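; Inventory item actor that the player picks up with E, adding its data to the ControlRef inventory under its row name and then destroying itself.
; Construction loads item info and basic info from data table rows, then initializes the state map and current state.
; ChangeState compares the current and previous states' bool and mesh maps, writing the comparison results into the StateSync maps.
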(event `self.ReceiveBeginPlay`
  (`|ExecutionSequence`
    (:`then_0`
      (`parent.ReceiveBeginPlay`))
    (:`then_1`
      (`self.Bind Event`))))

(event `Bind Event`
  (add `self.Key` (delegate `UpdateKey`)))

(event `UpdateKey` :!signature `self.Key`
  (params (Key :type "/Game/ProjectZeroCore/KeyRemappingSys/E_KeyBinding Enum") (`IsRelease?` :type Boolean))
  (bind _info (`self.Info`))
  (switch `/Game/ProjectZeroCore/KeyRemappingSys/E_KeyBinding` Key
    (:`NewEnumerator20`
      (`/Game/ProjectZeroAssets/Blueprints/Players/Player_PlayerController.AddItem` (`self.ControlRef`) (`KismetStringLibrary.Conv_NameToString` (`.RowName` (break `DataTableRowHandle` (`.Row_2_7C05D06DF844993DED8CC3908A4D9726` (break `/Game/ProjectZeroCore/InventorySys/S_Item` _info))))) _info)
      (`self.K2_DestroyActor`))))

(fn `ChangeBoolMap_0`
  (params (Key :type "/Game/ProjectZeroCore/InventorySys/E_ItemBool Enum") (Value :type Boolean))
  (`BlueprintMapLibrary.Map_Add` (`.BoolMap_4_DA8BA8A5B1450D01E66888AD570BCA9D` (break `/Game/ProjectZeroCore/InventorySys/S_ItemState` (`self.StateSync_0`))) Key Value))

(fn `ChangeState`
  (bind _currentstate_0 (`self.CurrentState_0`))
  (bind _info (`self.Info`))
  (bind ((`BasicInfo_76_C4DD2E1CC94D87B4AD6AD8A01F2CD0C7` _basicinfo) (`StateMap_66_3DD140BE984623EEA3DA61822DB3479D` _statemap) (`CurrentState_69_F00D0E2B8E4B9C2A9D25509A116A4743` _currentstate)) (break `/Game/ProjectZeroCore/InventorySys/S_Item` _info))
  (bind (_boolmap _meshmap) (break `/Game/ProjectZeroCore/InventorySys/S_ItemState` (`self.StateSync_0`)))
  (bind (_boolmap_2 _meshmap_2) (break `/Game/ProjectZeroCore/InventorySys/S_ItemState` (`BlueprintMapLibrary.Map_Find` _statemap (`self.LastState`))))
  (bind (_boolmap_3 _meshmap_3) (break `/Game/ProjectZeroCore/InventorySys/S_ItemState` (`BlueprintMapLibrary.Map_Find` _statemap _currentstate_0)))
  (set `self.LastState` _currentstate)
  (setmembers `/Game/ProjectZeroCore/InventorySys/S_Item` :`StructRef` _info :`CurrentState` _currentstate_0)
  (bind (_key _value) (`/Game/ProjectZeroCore/Utils/ActorMacros.CompareBoolMap` _boolmap_3 _boolmap_2)
    (:`Then`
      (`BlueprintMapLibrary.Map_Add` _boolmap (cast `/Game/ProjectZeroCore/InventorySys/E_ItemBool` _key) _value))
    (:`Complete`
      (bind (_key_2 _value_2) (`/Game/ProjectZeroCore/Utils/ActorMacros.CompareMeshMap` _meshmap_3 _meshmap_2)
        (:`Then`
          (`BlueprintMapLibrary.Map_Add` _meshmap (cast `/Game/ProjectZeroCore/InventorySys/E_ItemMesh` _key_2) _value_2))
        (:`Completed`
          (return))))))

(fn `UserConstructionScript`
  (bind _out_row (`/Game/ProjectZeroCore/Utils/ObjMacros.GetRow` (`.Row_2_7C05D06DF844993DED8CC3908A4D9726` (break `/Game/ProjectZeroCore/InventorySys/S_Item` (`self.Info`)))))
  (bind _output_get (set `self.Info` _out_row))
  (`|ExecutionSequence`
    (:`then_0`
      (bind ((`BasicInfo_76_C4DD2E1CC94D87B4AD6AD8A01F2CD0C7` _basicinfo) (`StateMap_66_3DD140BE984623EEA3DA61822DB3479D` _statemap) (`State_73_4D649F467E4716F315B4B6B9EC505930` _state) (`CurrentState_69_F00D0E2B8E4B9C2A9D25509A116A4743` _currentstate)) (break `/Game/ProjectZeroCore/InventorySys/S_Item` _output_get))
      (bind _out_row_2 (`/Game/ProjectZeroCore/Utils/ObjMacros.GetRow` _basicinfo))
      (set `self.BasicInfo` _out_row_2)
      (`parent.UserConstructionScript`))
    (:`then_1`
      (set `self.StateMap_0` _statemap)
      (set `self.CurrentState_0` _currentstate)
      (`self.ChangeState`))))