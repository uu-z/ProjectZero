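; Loot inventory Blueprint that fills its inventory component with randomized items from row-driven data during construction.
; The construction script loads its info row, sets the synced state from the current state, then loads basic info before running the parent script.
; It then loops over the loot list, rolls each entry's chance, writes a random min-to-max integer into the item's state and adds successful items to the inventory.
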(fn `UserConstructionScript`
  (bind _out_row (`/Game/ProjectZeroCore/Utils/ObjMacros.GetRow` (`.Row_6_5438E2127D481E649B13618DACB6E238` (break `/Game/ProjectZeroCore/InventorySys/S_Loot` (`self.Info`)))))
  (bind _output_get (set `self.Info` _out_row))
  (`|ExecutionSequence`
    (:`then_0`
      (bind ((`BasicInfo_50_1F952F69B24860DDC88656A640B5F369` _basicinfo) (`LootList_23_1473ED85F1471A5A62381AAF8773B973` _lootlist) (`CurrentState_18_C01E206BFC47C18356A471954ADB3095` _currentstate) (`StateMap_22_DA12DD3FE049F20D2EB44DB2AEB54415` _statemap)) (break `/Game/ProjectZeroCore/InventorySys/S_Loot` _output_get))
      (bind _output_get_2 (set `self.StateMap_0` _statemap))
      (bind _output_get_3 (set `self.CurrentState_0` _currentstate))
      (set `self.StateSync_0` (`BlueprintMapLibrary.Map_Find` _output_get_2 _output_get_3)))
    (:`then_1`
      (bind _out_row_2 (`/Game/ProjectZeroCore/Utils/ObjMacros.GetRow` _basicinfo))
      (set `self.BasicInfo` _out_row_2)
      (`parent.UserConstructionScript`))
    (:`then_2`
      (for _array_element _lootlist
        (bind (_row _intmap _floatmap) (break `/Game/ProjectZeroCore/InventorySys/S_LootItem` _array_element))
        (bind (_out_row_3 _returnvalue) (`/Game/ProjectZeroCore/Utils/ObjMacros.GetRow` _row))
        (`/Game/ProjectZeroCore/Utils/ObjMacros.ChanceExec` (`BlueprintMapLibrary.Map_Find` _floatmap "NewEnumerator1")
          (:`true`
            (`|ExecutionSequence`
              (:`then_0`
                (`BlueprintMapLibrary.Map_Add` (`.IntMap_16_5E024D6D524B4D6202191CB6B82F4C76` (break `/Game/ProjectZeroCore/InventorySys/S_ItemState` (`.State_73_4D649F467E4716F315B4B6B9EC505930` (break `/Game/ProjectZeroCore/InventorySys/S_Item` _out_row_3)))) "NewEnumerator1" (`KismetMathLibrary.RandomIntegerInRange` (`BlueprintMapLibrary.Map_Find` _intmap "NewEnumerator1") (`BlueprintMapLibrary.Map_Find` _intmap "NewEnumerator2"))))
              (:`then_1`
                (`/Game/ProjectZeroAssets/Blueprints/Inventory/InventoryComponent.AddItem` (`self.InventoryComponent`) _returnvalue _out_row_3)))))))))