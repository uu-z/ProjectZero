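; Inventory container Blueprint whose construction script begins building loot from data table rows.
; It refreshes its Info struct from the referenced row, then looks up each listed item's row and runs a chance roll using that entry's float map value.
; Loot generation is unfinished: the inventory component's AddItem call is unreachable, and the random quantity and LootMap nodes are unused, so no items are added.
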(fn `UserConstructionScript`
  (bind _out_row (`/Game/ProjectZeroCore/Utils/ObjMacros.GetRow` (`.Row_6_5438E2127D481E649B13618DACB6E238` (break `/Game/ProjectZeroCore/InventorySys/S_Loot` (`self.Info`)))))
  (bind _output_get (set `self.Info` _out_row))
  (`|ExecutionSequence`
    (:`then_0`
      (for _array_element (`.Item_3_1473ED85F1471A5A62381AAF8773B973` (break `/Game/ProjectZeroCore/InventorySys/S_Loot` _output_get))
        (bind (_row _intmap _floatmap) (break `/Game/ProjectZeroCore/InventorySys/S_LootItem` _array_element))
        (bind _out_row_2 (`/Game/ProjectZeroCore/Utils/ObjMacros.GetRow` _row))
        (`/Game/ProjectZeroCore/Utils/ObjMacros.ChanceExec` (`BlueprintMapLibrary.Map_Find` _floatmap "NewEnumerator1"))))))