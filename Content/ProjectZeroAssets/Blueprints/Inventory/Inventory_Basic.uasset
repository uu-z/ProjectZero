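; Base inventory item actor whose static mesh and custom-depth rendering are driven by data-table state.
; Construction loads its row and copies the current state's entry into StateSync.
; InteractionComponent delivers key presses, which are only printed, and operators, whose "=" rows overwrite matching StateSync bools.
; Tick compares StateSync's mesh and bool maps against BasicInfo.State, raising update events that apply changes to the StaticMesh.
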(event `Event Bind`
  (bind _interactioncomponent (`self.InteractionComponent`))
  (add `/InteractionSys/Core/InteractionComponent.Key` _interactioncomponent (delegate `Key_Event_0`))
  (add `/InteractionSys/Core/InteractionComponent.Operator` _interactioncomponent (delegate `Operator_Event_0`))
  (add `self.UpdateMesh` (delegate `UpdateMesh_Event`))
  (add `self.UpdateBool` (delegate `UpdateBool_Event`)))

(event `Key_Event_0`
  (params (Key :type "/InteractionSys/Core/E_KeyBinding Enum") (`IsRelease?` :type Boolean) (Ref :type "/InteractionSys/Core/InteractionComponent Object Reference"))
  (`/ren/Utils/ObjMacros.CheckInput` `IsRelease?`
    (:`Press`
      (`KismetSystemLibrary.PrintString` (`|GetEnumeratorNameAsString` Key)))))

(event `self.ReceiveBeginPlay`
  (`self.Event Bind`))

(event `Operator_Event_0`
  (params (Operator :type "/Game/ProjectZeroCore/CommandSys/S_Operator Structure"))
  (bind (_meshmap _boolmap) (break `/Game/ProjectZeroCore/InventorySys/S_INState` (`self.StateSync`)))
  (for _array_element (`.Operators_4_321192DC2D4273012FB6DA8A69BB2CBF` (break `/Game/ProjectZeroCore/CommandSys/S_Operator` Operator))
    (bind _out_row (`/ren/Utils/ObjMacros.GetRow` _array_element))
    (bind (_operator _boolmap_2) (break `/InteractionSys/Core/S_Operator` _out_row))
    (switch `/InteractionSys/Core/E_Operator` _operator
      (:`NewEnumerator1`
        (bind _key (`/ren/Utils/ObjMacros.ByteQueue` _boolmap)
          (:`Then`
            (bind _returnvalue (cast `/Game/ProjectZeroCore/InventorySys/E_INBool` _key))
            (bind (_value _returnvalue_2) (`BlueprintMapLibrary.Map_Find` _boolmap_2 (`|GetEnumeratorNameAsString` _returnvalue)))
            (if _returnvalue_2
              (`BlueprintMapLibrary.Map_Add` _boolmap _returnvalue _value))))))))

(event `self.ReceiveTick`
  (params (DeltaSeconds :type "Float (single-precision)"))
  (bind (_meshmap _boolmap) (break `/Game/ProjectZeroCore/InventorySys/S_INState` (`self.StateSync`)))
  (bind (_meshmap_2 _boolmap_2) (break `/Game/ProjectZeroCore/InventorySys/S_INState` (`.State_17_AAB1864CC543F7B19E1D7FB6E717B925` (break `/Game/ProjectZeroCore/InventorySys/S_IN` (`self.BasicInfo`)))))
  (`|ExecutionSequence`
    (:`then_0`
      (bind (_key _value) (`/ren/Utils/ObjMacros.Sync_ByteMeshMap` _meshmap _meshmap_2)
        (:`then`
          (`self.UpdateMesh` (cast `/Game/ProjectZeroCore/InventorySys/E_INMesh` _key) _value))
        (:`Completed`
          (bind (_key_2 _value_2) (`/ren/Utils/ObjMacros.Sync_ByteBoolMap` _boolmap _boolmap_2)
            (:`Then`
              (`self.UpdateBool` (cast `/Game/ProjectZeroCore/InventorySys/E_INBool` _key_2) _value_2))))))))

(event `UpdateMesh_Event` :!signature `self.UpdateMesh`
  (params (Key :type "/Game/ProjectZeroCore/InventorySys/E_INMesh Enum") (Value :type "StaticMesh Object Reference"))
  (switch `/Game/ProjectZeroCore/InventorySys/E_INMesh` Key
    (:`NewEnumerator1`
      (`StaticMeshComponent.SetStaticMesh` (`self.StaticMesh`) Value))))

(event `UpdateBool_Event` :!signature `self.UpdateBool`
  (params (Key :type "/Game/ProjectZeroCore/InventorySys/E_INBool Enum") (Value :type Boolean))
  (switch `/Game/ProjectZeroCore/InventorySys/E_INBool` Key
    (:`NewEnumerator1`
      (`PrimitiveComponent.SetRenderCustomDepth` (`self.StaticMesh`) Value))))

(fn `ChangeBoolMap`
  (params (Key :type "/Game/ProjectZeroCore/InventorySys/E_INBool Enum") (Value :type Boolean))
  (`BlueprintMapLibrary.Map_Add` (`.BoolMap_9_A32C1619FD42EC07CC6E578AE771053F` (break `/Game/ProjectZeroCore/InventorySys/S_INState` (`self.StateSync`))) Key Value))

(fn `GetRegisterName`
  (returns (Name :type Name))
  (return (`KismetStringLibrary.Conv_StringToName` (`KismetSystemLibrary.GetDisplayName` self))))

(fn `UserConstructionScript`
  (bind _out_row (`/ren/Utils/ObjMacros.GetRow` (`.Row_14_497070799C471DCC82986EAD46FBA5EF` (break `/Game/ProjectZeroCore/InventorySys/S_IN` (`self.BasicInfo`)))))
  (bind _output_get (set `self.BasicInfo` _out_row))
  (`|ExecutionSequence`
    (:`then_0`
      (bind ((`State_17_AAB1864CC543F7B19E1D7FB6E717B925` _state) (`CurrentState_22_56B741A4CA4FAF578D1B15B675F05D11` _currentstate) (`StateMap_26_0CEADA2ABE418DCF2B32B3AE352B17E6` _statemap)) (break `/Game/ProjectZeroCore/InventorySys/S_IN` _output_get))
      (bind _output_get_2 (set `self.StateMap` _statemap))
      (bind _output_get_3 (set `self.CurrentState` _currentstate))
      (set `self.StateSync` (`BlueprintMapLibrary.Map_Find` _output_get_2 _output_get_3)))))