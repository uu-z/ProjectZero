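; Base game state actor that loads its state and control settings from a row and coordinates global state, manager actors and interaction commands.
; Tick syncs bool, float and manager maps against Info, firing update calls for synced entries, and flushes queued unlocks.
; Update handlers set global time dilation and lazily spawn managers by class, forwarding control toggles and dropping destroyed ones.
; Interaction components register by key so CallCommand can route commands by name.
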(event `Bind Event`
  (add `self.UpdateFloat` (delegate `UpdateFloat_Event`))
  (add `self.UpdateManager` (delegate `UpdateCtrlClass_Event`)))

(event `UpdateFloat_Event` :!signature `self.UpdateFloat`
  (params (Key :type "/Game/ProjectZeroCore/GameSys/E_GameStateFloat Enum") (Value :type "Float (double-precision)"))
  (switch `/Game/ProjectZeroCore/GameSys/E_GameStateFloat` Key
    (:`NewEnumerator1`
      (`GameplayStatics.SetGlobalTimeDilation` Value))))

(event `self.ReceiveBeginPlay`
  (`self.Bind Event`))

(event `UpdateCtrlClass_Event` :!signature `self.UpdateManager`
  (params (Key :type "/Game/ProjectZeroAssets/Blueprints/Game/Manager/Manager_Basic Class Reference") (Value :type Boolean))
  (bind _managerrefmap (`self.ManagerRefMap`))
  (bind (_value _returnvalue) (`BlueprintMapLibrary.Map_Find` _managerrefmap Key))
  (if Value
    (if _returnvalue
      (`/Game/ProjectZeroAssets/Blueprints/Game/Manager/Manager_Basic.OnCtrl` _value Value)
      (else
        (bind _returnvalue_2 (`|SpawnActorFromClass` Key (`self.GetTransform`) "Undefined" "OverrideRootScale"))
        (`/Game/ProjectZeroAssets/Blueprints/Game/Manager/Manager_Basic.OnCtrl` _returnvalue_2 Value)
        (add `/Game/ProjectZeroAssets/Blueprints/Game/Manager/Manager_Basic.Destory` _returnvalue_2 (delegate `CustomEvent_0`))
        (`BlueprintMapLibrary.Map_Add` _managerrefmap Key _returnvalue_2)))
    (elif _returnvalue
      (`/Game/ProjectZeroAssets/Blueprints/Game/Manager/Manager_Basic.OnCtrl` _value Value))))

(event `self.ReceiveTick`
  (params (DeltaSeconds :type "Float (single-precision)"))
  (bind _unlockmap (`self.UnLockMap`))
  (bind ((`__State_37_499E9FA6AC4DC6FCE31F20B06CE46D59` ___state) (`__GameCtrl_38_7E00309FF54A8D840AA201A6E8D8D822` ___gamectrl)) (break `/Game/ProjectZeroCore/GameSys/S_GameInfo` (`self.info`)))
  (bind (_boolmap _floatmap) (break `/Game/ProjectZeroCore/GameSys/S_GameState` (`self.StateSync`)))
  (bind (_ctrlmap _managers) (break `/Game/ProjectZeroCore/GameSys/S_GameCtrl` (`self.CtrlSync`)))
  (bind (_boolmap_2 _floatmap_2) (break `/Game/ProjectZeroCore/GameSys/S_GameState` ___state))
  (bind (_ctrlmap_2 _managers_2) (break `/Game/ProjectZeroCore/GameSys/S_GameCtrl` ___gamectrl))
  (`|ExecutionSequence`
    (:`then_0`
      (bind (_key _value) (`/Game/ProjectZeroCore/Utils/ObjMacros.SyncBoolMap` _boolmap _boolmap_2)
        (:`Then`
          (`self.UpdateBool` (cast `/Game/ProjectZeroCore/GameSys/E_GameCtrlBool` _key) _value))
        (:`Completed`
          (bind (_key_2 _value_2) (`/Game/ProjectZeroCore/Utils/ObjMacros.SyncFloatMap` _floatmap _floatmap_2)
            (:`then`
              (`self.UpdateFloat` (cast `/Game/ProjectZeroCore/GameSys/E_GameStateFloat` _key_2) _value_2))
            (:`Completed`
              (bind (_key_3 _value_3) (`/Game/ProjectZeroCore/Utils/ObjMacros.SyncStringBoolMap` _ctrlmap _ctrlmap_2)
                (:`then`
                  (`self.UpdateCtrlBool` _key_3 _value_3))
                (:`Completed`
                  (bind (_array_element _value_4) (`/Game/ProjectZeroCore/Utils/ObjMacros.SyncClassBoolMap` _managers _managers_2)
                    (:`Then`
                      (bind _asmanager_basic (castclass `/Game/ProjectZeroAssets/Blueprints/Game/Manager/Manager_Basic` _array_element))
                      (`self.UpdateManager` _asmanager_basic _value_4))))))))))
    (:`then_1`
      (for _array_element_2 _unlockmap
        (`self.UnLock` _array_element_2))
      (`KismetArrayLibrary.Array_Clear` _unlockmap))))

(event `CustomEvent_0`
  (params (Class :type "/Game/ProjectZeroAssets/Blueprints/Game/Manager/Manager_Basic Class Reference"))
  (`BlueprintMapLibrary.Map_Remove` (`self.ManagerRefMap`) Class))

(fn `CallCommand`
  (params (Name :type String) (Commands :type String))
  (bind (_value _returnvalue) (`BlueprintMapLibrary.Map_Find` (`self.InterActionMaps`) Name))
  (if _returnvalue
    (`/Game/ProjectZeroAssets/Blueprints/Components/Interaction/InteractionComponent.Command` _value Commands)
    (else
      (`KismetSystemLibrary.PrintString` "Command Ref Not Exists"))))

(fn `ChangeManager`
  (params (Key :type "/Game/ProjectZeroAssets/Blueprints/Game/Manager/Manager_Basic Class Reference") (Value :type Boolean)))

(fn `RegInteractionComponent`
  (params (Key :type "String (by ref)") (Value :type "/Game/ProjectZeroAssets/Blueprints/Components/Interaction/InteractionComponent Object Reference (by ref)"))
  (`BlueprintMapLibrary.Map_Add` (`self.InterActionMaps`) Key Value))

(fn `UserConstructionScript`
  (bind _out_row (`/Game/ProjectZeroCore/Utils/ObjMacros.GetRow` (`.Row_3_8EE1C8F8E14AA73FC4935B8B577D2A31` (break `/Game/ProjectZeroCore/GameSys/S_GameInfo` (`self.info`)))))
  (bind _output_get (set `self.info` _out_row))
  (`|ExecutionSequence`
    (:`then_0`
      (bind ((`CurrentState_6_0F30E07261435876861CF0B7DA99CF33` _currentstate) (`StateMap_36_4C480B2FEB4EB34798F76194A27131F0` _statemap) (`__State_37_499E9FA6AC4DC6FCE31F20B06CE46D59` ___state) (`CurCtrl_31_FB958AE14D4E5309D480B6913512F5DC` _curctrl) (`CtrlMap_35_E37E69E83C44034B3B9CF1B5E49DB969` _ctrlmap)) (break `/Game/ProjectZeroCore/GameSys/S_GameInfo` _output_get))
      (bind _output_get_2 (set `self.StateMapSync` _statemap))
      (bind _output_get_3 (set `self.CurrentStateSync` _currentstate))
      (set `self.StateSync` (`BlueprintMapLibrary.Map_Find` _output_get_2 _output_get_3)))
    (:`then_1`
      (bind _output_get_4 (set `self.CtrlMap` _ctrlmap))
      (bind _output_get_5 (set `self.CurCtrl` _curctrl))
      (set `self.CtrlSync` (`BlueprintMapLibrary.Map_Find` _output_get_4 _output_get_5)))))