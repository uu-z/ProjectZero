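; Base-style NPC controller that possesses an NPC_Basic pawn and registers its interaction component with GState_Base under the pawn's display name.
; Construction loads Info from a row and picks the StateSync entry for the current state from its state map.
; Tick syncs string, bool and float maps between StateSync and Info.State, calling update dispatchers with enum-converted keys.
; The bound update handlers are empty, and OnCommands and OnKey are stubs returning false.
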(event `Event Bind`
  (add `self.UpdateStateString` (delegate `UpdateStateString_Event`))
  (add `self.UpdateStateBool` (delegate `UpdateStateBool_Event`))
  (add `self.UpdateStateFloat` (delegate `UpdateStateFloat_Event`)))

(event `self.OnPossess`
  (params (PossessedPawn :type "Pawn Object Reference"))
  (`|ExecutionSequence`
    (:`then_0`
      (bind _asnpc_basic (cast `/Game/ProjectZeroAssets/Blueprints/NPC/NPC_Basic` PossessedPawn))
      (set `self.PawnRef` _asnpc_basic))
    (:`then_1`
      (bind _asgstate_base (cast `/Game/ProjectZeroAssets/Blueprints/Game/GState_Base` (`GameplayStatics.GetGameState`)))
      (`/Game/ProjectZeroAssets/Blueprints/Game/GState_Base.RegInteractionComponent` _asgstate_base (`KismetSystemLibrary.GetDisplayName` (`self.PawnRef`)) (`self.InteractionComponent`)))))

(event `UpdateStateString_Event` :!signature `self.UpdateStateString`
  (params (Key :type "/Game/ProjectZeroCore/NpcSys/E_NPCStateString Enum") (Value :type String)))

(event `UpdateStateBool_Event` :!signature `self.UpdateStateBool`
  (params (Key :type "/Game/ProjectZeroCore/NpcSys/E_NPCStateBool Enum") (Value :type Boolean)))

(event `self.ReceiveTick`
  (params (DeltaSeconds :type "Float (single-precision)"))
  (bind (_stringmap _boolmap _floatmap) (break `/Game/ProjectZeroCore/NpcSys/S_NPCState` (`self.StateSync`)))
  (bind (_stringmap_2 _boolmap_2 _floatmap_2) (break `/Game/ProjectZeroCore/NpcSys/S_NPCState` (`.__State_17_0BBEF7E1B3458EB3E5D978AE3A2010F5` (break `/Game/ProjectZeroCore/NpcSys/S_NPC` (`self.Info`)))))
  (`|ExecutionSequence`
    (:`then_0`
      (bind (_key _value) (`/Game/ProjectZeroCore/Utils/ObjMacros.SyncStringMap` _stringmap _stringmap_2)
        (:`Then`
          (`self.UpdateStateString` (cast `/Game/ProjectZeroCore/NpcSys/E_NPCStateString` _key) _value))
        (:`Completed`
          (bind (_key_2 _value_2) (`/Game/ProjectZeroCore/Utils/ObjMacros.SyncBoolMap` _boolmap _boolmap_2)
            (:`Then`
              (`self.UpdateStateBool` (cast `/Game/ProjectZeroCore/NpcSys/E_NPCStateBool` _key_2) _value_2))
            (:`Completed`
              (bind (_key_3 _value_3) (`/Game/ProjectZeroCore/Utils/ObjMacros.SyncFloatMap` _floatmap _floatmap_2)
                (:`then`
                  (`self.UpdateStateFloat` (cast `/Game/ProjectZeroCore/NpcSys/E_NPCStateFloat` _key_3) _value_3))))))))))

(event `UpdateStateFloat_Event` :!signature `self.UpdateStateFloat`
  (params (Key :type "/Game/ProjectZeroCore/NpcSys/E_NPCStateFloat Enum") (Value :type "Float (double-precision)")))

(fn `OnCommands`
  (params (CommandMap :type "Map of /Game/ProjectZeroCore/Utils/E_Operator Enum to /Game/ProjectZeroCore/Utils/S_Parse Structure"))
  (returns (NewParam :type Boolean))
  (return false))

(fn `OnKey`
  (params (Key :type "/Game/ProjectZeroCore/KeyRemappingSys/E_KeyBinding Enum" :default "NewEnumerator0") (Value :type Boolean) (Ref :type "/Game/ProjectZeroAssets/Blueprints/Components/Interaction/InteractionComponent Object Reference"))
  (returns (NewParam :type Boolean))
  (return false))

(fn `UserConstructionScript`
  (bind _out_row (`/Game/ProjectZeroCore/Utils/ObjMacros.GetRow` (`.Row_2_AB97FAD8D84F3A22F9F51D9F0BE09B58` (break `/Game/ProjectZeroCore/NpcSys/S_NPC` (`self.Info`)))))
  (bind _output_get (set `self.Info` _out_row))
  (`|ExecutionSequence`
    (:`then_0`
      (bind (_row _curstate _statemap) (break `/Game/ProjectZeroCore/NpcSys/S_NPC` _output_get))
      (bind _output_get_2 (set `self.StateMap` _statemap))
      (bind _output_get_3 (set `self.CurState` _curstate))
      (set `self.StateSync` (`BlueprintMapLibrary.Map_Find` _output_get_2 _output_get_3)))))