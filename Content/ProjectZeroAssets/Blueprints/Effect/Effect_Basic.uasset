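; Base effect actor that applies float and bool state changes to the player controller, optionally repeated, and destroys itself when repeats run out.
; Construction loads the effect's state and control-state maps from a row lookup.
; While CanTick is set, Tick reads control flags as triggers: ListenState pushes additive and set values to the player, ListenControl syncs control bools.
; In Do N mode, the listen-end event delays, decrements the count and re-arms ListenState.
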(event `Event Bind`
  (`|ExecutionSequence`
    (:`then_0`
      (add `self.OnListenStateEnd` (delegate `OnListenStateEnd_Event`)))))

(event `self.ReceiveBeginPlay`
  (`|ExecutionSequence`
    (:`then_0`
      (bind _asplayer_player_controller (cast `/Game/ProjectZeroAssets/Blueprints/Players/Player_PlayerController` (`GameplayStatics.GetPlayerController` 0)))
      (set `self.ControlRef` _asplayer_player_controller))
    (:`then_1`
      (`self.Event Bind`))))

(event `OnListenStateEnd_Event`
  (bind (_boolmap _floatmap _enummap) (break `/Game/ProjectZeroCore/EffectSys/S_EffectCtrlState` (`self.CtrlStateSync`)))
  (bind (_value _returnvalue) (`BlueprintMapLibrary.Map_Find` _enummap "NewEnumerator1"))
  (bind (_value_2 _returnvalue_2) (`BlueprintMapLibrary.Map_Find` _floatmap "NewEnumerator1"))
  (bind (_value_3 _returnvalue_3) (`BlueprintMapLibrary.Map_Find` _floatmap "NewEnumerator2"))
  (switch `/Game/ProjectZeroCore/EffectSys/E_EffectCtrlEnumValue` _value
    (:`NewEnumerator2`
      (if (and _returnvalue _returnvalue_2 _returnvalue_3 (> _value_2 0.0))
        (`KismetSystemLibrary.Delay` _value_3)
        (`self.ChangeCtrlFloat` "NewEnumerator1" (- _value_2 1.0))
        (`self.ChangeCtrlBool` "NewEnumerator3" true)
        (else
          (`self.K2_DestroyActor`))))))

(event `self.ReceiveTick`
  (params (DeltaSeconds :type "Float (single-precision)"))
  (bind ((`Class_93_1EE3FCBBE446E2152661DBA9E3660676` _class) (`State_71_DB48E7C43D43571B06E8D28636101E06` _state) (`ControlState_88_075E761485484F9D8E761DBD390C053E` _controlstate)) (break `/Game/ProjectZeroCore/EffectSys/S_Effect` (`self.Info`)))
  (bind _boolmap (break `/Game/ProjectZeroCore/EffectSys/S_EffectCtrlState` (`self.CtrlStateSync`)))
  (bind (_boolmap_2 _floatmap) (break `/Game/ProjectZeroCore/PlayerSys/S_PlayerState` (`/Game/ProjectZeroAssets/Blueprints/Players/Player_PlayerController.StateSync` (`self.ControlRef`))))
  (bind (_addfloat _setfloat _setbool) (break `/Game/ProjectZeroCore/EffectSys/S_EffectPlayer` (`.Player_10_29111BA11F43F9F3236A5BB7581711A4` (break `/Game/ProjectZeroCore/EffectSys/S_EffectState` (`self.StateSync`)))))
  (bind (_value _returnvalue) (`BlueprintMapLibrary.Map_Find` _boolmap "NewEnumerator1"))
  (bind (_addfloat_2 _setfloat_2 _setbool_2) (break `/Game/ProjectZeroCore/EffectSys/S_EffectPlayer` (`.Player_10_29111BA11F43F9F3236A5BB7581711A4` (break `/Game/ProjectZeroCore/EffectSys/S_EffectState` _state))))
  (`/Game/ProjectZeroCore/Utils/ObjMacros.AndTrueExec` _value _returnvalue
    (:`true`
      (bind (_key _value_2) (`/Game/ProjectZeroCore/Utils/ObjMacros.ByteQueue` _boolmap)
        (:`Then`
          (`/Game/ProjectZeroCore/Utils/ObjMacros.AndTrueExec` _value_2 true
            (:`true`
              (switch `/Game/ProjectZeroCore/EffectSys/E_EffectCtrlBool` (cast `/Game/ProjectZeroCore/EffectSys/E_EffectCtrlBool` _key)
                (:`NewEnumerator3`
                  (`self.OnListenStateStart`)
                  (`/Game/ProjectZeroCore/Utils/ObjMacros.SyncFloatMap` _addfloat _addfloat_2
                    (:`Completed`
                      (`/Game/ProjectZeroCore/Utils/ObjMacros.SyncIncFloatMap` _addfloat_2 _floatmap
                        (:`Completed`
                          (`/Game/ProjectZeroCore/Utils/ObjMacros.SyncFloatMap` _setfloat _setfloat_2
                            (:`Completed`
                              (`/Game/ProjectZeroCore/Utils/ObjMacros.SyncFloatMap` _floatmap _floatmap
                                (:`Completed`
                                  (`/Game/ProjectZeroCore/Utils/ObjMacros.SyncBoolMap` _setbool _setbool_2
                                    (:`Completed`
                                      (`/Game/ProjectZeroCore/Utils/ObjMacros.SyncBoolMap` _setbool_2 _boolmap_2
                                        (:`Completed`
                                          (`self.ChangeCtrlBool` "NewEnumerator3")
                                          (`self.OnListenStateEnd`))))))))))))))
                (:`NewEnumerator4`
                  (`/Game/ProjectZeroCore/Utils/ObjMacros.SyncBoolMap` (`.BoolMap_9_EA24D7704646C16FC59B0DAAFDB7E4B0` (break `/Game/ProjectZeroCore/EffectSys/S_EffectCtrlState` (`self.CtrlStateSync`))) (`.BoolMap_9_EA24D7704646C16FC59B0DAAFDB7E4B0` (break `/Game/ProjectZeroCore/EffectSys/S_EffectCtrlState` _controlstate))
                    (:`Completed`
                      (`self.ChangeCtrlBool` "NewEnumerator4"))))))))))))

(fn `ChangeCtrlBool`
  (params (Key :type "/Game/ProjectZeroCore/EffectSys/E_EffectCtrlBool Enum") (Value :type Boolean))
  (bind _boolmap (break `/Game/ProjectZeroCore/EffectSys/S_EffectCtrlState` (`self.CtrlStateSync`)))
  (`BlueprintMapLibrary.Map_Add` _boolmap Key Value)
  (`BlueprintMapLibrary.Map_Add` _boolmap "NewEnumerator4" true))

(fn `ChangeCtrlFloat`
  (params (Key :type "/Game/ProjectZeroCore/EffectSys/E_EffectCtrlFloat Enum") (Value :type "Float (double-precision)"))
  (bind (_boolmap _floatmap) (break `/Game/ProjectZeroCore/EffectSys/S_EffectCtrlState` (`self.CtrlStateSync`)))
  (`BlueprintMapLibrary.Map_Add` _floatmap Key Value)
  (`BlueprintMapLibrary.Map_Add` _boolmap "NewEnumerator4"))

(fn `UserConstructionScript`
  (bind _out_row (`/Game/ProjectZeroCore/Utils/ObjMacros.GetRow` (`.Row_57_7BC961FDB74510BD1DD50CB953F40697` (break `/Game/ProjectZeroCore/EffectSys/S_Effect` (`self.Info`)))))
  (bind _output_get (set `self.Info` _out_row))
  (`|ExecutionSequence`
    (:`then_0`
      (bind (_row _class _statemap _currentstate _state _controlstatemap _currentcontrolstate) (break `/Game/ProjectZeroCore/EffectSys/S_Effect` _output_get))
      (bind _output_get_2 (set `self.StateMap` _statemap))
      (bind _output_get_3 (set `self.CurState` _currentstate))
      (set `self.StateSync` (`BlueprintMapLibrary.Map_Find` _output_get_2 _output_get_3)))
    (:`then_1`
      (bind _output_get_4 (set `self.CtrlStateMap` _controlstatemap))
      (bind _output_get_5 (set `self.CurCtrlState` _currentcontrolstate))
      (set `self.CtrlStateSync` (`BlueprintMapLibrary.Map_Find` _output_get_4 _output_get_5)))))