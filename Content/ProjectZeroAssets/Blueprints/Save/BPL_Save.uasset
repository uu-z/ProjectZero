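; Blueprint function library that loads, saves and resets save data for key mappings and unlock info.
; Key mappings load from their save slot or fall back to defaults built from action and axis input DataTables, flagging when no save exists.
; Saves update the existing slot object or create one.
; Unlock slot names come from the info's string map; unlock loading has no fallback, and its default function is empty.
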(fn `LoadDefaultKeyMapping`
  (returns (info1 :type "/Game/ProjectZeroCore/KeyRemappingSys/S_KeyMapping Structure"))
  (locals (KeyMapping :type "/Game/ProjectZeroCore/KeyRemappingSys/S_KeyMapping Structure"))
  (bind (_saveslot _actioninputs _axisinputs) (break `/Game/ProjectZeroCore/KeyRemappingSys/S_KeyMapping` (`local.KeyMapping`)))
  (`|ExecutionSequence`
    (:`then_0`
      (bind _outrownames (`DataTableFunctionLibrary.GetDataTableRowNames` "/Game/ProjectZeroAssets/Blueprints/Save/T_DefaultActionInput.T_DefaultActionInput"))
      (for _array_element _outrownames
        (bind _returnvalue (`|GetDataTableRow` "/Game/ProjectZeroAssets/Blueprints/Save/T_DefaultActionInput.T_DefaultActionInput" _array_element)
          (:`then`
            (`KismetArrayLibrary.Array_Add` _actioninputs _returnvalue)))))
    (:`then_1`
      (bind _outrownames_2 (`DataTableFunctionLibrary.GetDataTableRowNames` "/Game/ProjectZeroAssets/Blueprints/Save/T_DefaultAxisInput.T_DefaultAxisInput"))
      (for _array_element_2 _outrownames_2
        (bind _returnvalue_2 (`|GetDataTableRow` "/Game/ProjectZeroAssets/Blueprints/Save/T_DefaultAxisInput.T_DefaultAxisInput" _array_element_2)
          (:`then`
            (`KismetArrayLibrary.Array_Add` _axisinputs _returnvalue_2)))))
    (:`then_2`
      (return (`local.KeyMapping`)))))

(fn `LoadDefaultUnLock`
  (returns (info :type "/Game/ProjectZeroCore/UnlockSys/S_Unlock Structure"))
  (return))

(fn `LoadKeyMapping`
  (returns (Info :type "/Game/ProjectZeroCore/KeyRemappingSys/S_KeyMapping Structure") (`NoSave?` :type Boolean))
  (locals (KeyMapping :type "/Game/ProjectZeroCore/KeyRemappingSys/S_KeyMapping Structure"))
  (bind _saveslot (break `/Game/ProjectZeroCore/KeyRemappingSys/S_KeyMapping` (`local.KeyMapping`)))
  (bind _returnvalue (`GameplayStatics.DoesSaveGameExist` _saveslot))
  (if _returnvalue
    (bind _returnvalue_2 (`GameplayStatics.LoadGameFromSlot` _saveslot))
    (bind _assave_key_mapping (cast `/Game/ProjectZeroAssets/Blueprints/Save/Save_KeyMapping` _returnvalue_2))
    (return (`/Game/ProjectZeroAssets/Blueprints/Save/Save_KeyMapping.KeyMappingInfo` _assave_key_mapping) false)
    (else
      (bind _info1 (`self.LoadDefaultKeyMapping` null))
      (return _info1 true))))

(fn `LoadUnlock`
  (params (UserIndex :type Integer))
  (returns (UnlockInfo1 :type "/Game/ProjectZeroCore/UnlockSys/S_Unlock Structure"))
  (locals (UnLockInfo :type "/Game/ProjectZeroCore/UnlockSys/S_Unlock Structure"))
  (bind _value (`BlueprintMapLibrary.Map_Find` (`.StringMap_6_3426C11E9B485EE794718681E0CACAEE` (break `/Game/ProjectZeroCore/UnlockSys/S_Unlock` (`local.UnLockInfo`))) "NewEnumerator1"))
  (bind _returnvalue (`GameplayStatics.DoesSaveGameExist` _value UserIndex))
  (if _returnvalue
    (bind _returnvalue_2 (`GameplayStatics.LoadGameFromSlot` _value UserIndex))
    (bind _assave_unlock (cast `/Game/ProjectZeroAssets/Blueprints/Save/Save_Unlock` _returnvalue_2))
    (return (`/Game/ProjectZeroAssets/Blueprints/Save/Save_Unlock.UnlockInfo` _assave_unlock))))

(fn `ResetKeyMapping`
  (bind _info1 (`self.LoadDefaultKeyMapping` null))
  (`self.SaveKeyMapping` _info1))

(fn `ResetUnLock`
  (bind _info (`self.LoadDefaultUnLock` null))
  (`self.SaveUnLock` _info))

(fn `SaveKeyMapping`
  (params (Info :type "/Game/ProjectZeroCore/KeyRemappingSys/S_KeyMapping Structure"))
  (bind _saveslot (break `/Game/ProjectZeroCore/KeyRemappingSys/S_KeyMapping` Info))
  (bind _returnvalue (`GameplayStatics.DoesSaveGameExist` _saveslot))
  (if _returnvalue
    (bind _returnvalue_2 (`GameplayStatics.LoadGameFromSlot` _saveslot))
    (bind _assave_key_mapping (cast `/Game/ProjectZeroAssets/Blueprints/Save/Save_KeyMapping` _returnvalue_2))
    (set `/Game/ProjectZeroAssets/Blueprints/Save/Save_KeyMapping.KeyMappingInfo` Info _assave_key_mapping)
    (`GameplayStatics.SaveGameToSlot` _returnvalue_2 _saveslot)
    (else
      (bind _returnvalue_3 (`GameplayStatics.CreateSaveGameObject` "/Game/ProjectZeroAssets/Blueprints/Save/Save_KeyMapping.Save_KeyMapping_C"))
      (set `/Game/ProjectZeroAssets/Blueprints/Save/Save_KeyMapping.KeyMappingInfo` Info _returnvalue_3)
      (`GameplayStatics.SaveGameToSlot` _returnvalue_3 _saveslot))))

(fn `SaveUnLock`
  (params (info :type "/Game/ProjectZeroCore/UnlockSys/S_Unlock Structure") (UserIndex :type Integer))
  (bind _value (`BlueprintMapLibrary.Map_Find` (`.StringMap_6_3426C11E9B485EE794718681E0CACAEE` (break `/Game/ProjectZeroCore/UnlockSys/S_Unlock` info)) "NewEnumerator1"))
  (bind _returnvalue (`GameplayStatics.DoesSaveGameExist` _value UserIndex))
  (if _returnvalue
    (bind _returnvalue_2 (`GameplayStatics.LoadGameFromSlot` _value UserIndex))
    (bind _assave_unlock (cast `/Game/ProjectZeroAssets/Blueprints/Save/Save_Unlock` _returnvalue_2))
    (set `/Game/ProjectZeroAssets/Blueprints/Save/Save_Unlock.UnlockInfo` info _assave_unlock)
    (`GameplayStatics.SaveGameToSlot` _assave_unlock _value UserIndex)
    (else
      (bind _returnvalue_3 (`GameplayStatics.CreateSaveGameObject` "/Game/ProjectZeroAssets/Blueprints/Save/Save_Unlock.Save_Unlock_C"))
      (set `/Game/ProjectZeroAssets/Blueprints/Save/Save_Unlock.UnlockInfo` info _returnvalue_3)
      (`GameplayStatics.SaveGameToSlot` _returnvalue_3 _value UserIndex))))