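; Blueprint library that loads and saves the player's key mapping of action and axis inputs.
; LoadDefaultMapping builds the mapping Info from the rows of the default action and axis input data tables.
; SaveMapping writes Info into a BP_Save slot, updating the existing save or creating one.
; LoadMapping checks for a "Player" save but always returns the defaults with NoSave true, as its saved-game branch is disconnected.
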(fn `LoadDefaultMapping`
  (returns (info1 :type "/Game/ProjectZeroCore/KeyRemappingSys/S_Save Structure"))
  (locals (info :type "/Game/ProjectZeroCore/KeyRemappingSys/S_Save Structure"))
  (bind (_actioninputs _axisinputs) (break `/Game/ProjectZeroCore/KeyRemappingSys/S_Save` (`local.info`)))
  (`|ExecutionSequence`
    (:`then_0`
      (bind _outrownames (`DataTableFunctionLibrary.GetDataTableRowNames` "/Game/ProjectZeroAssets/Blueprints/KeyMapping/T_DefaultActionInput.T_DefaultActionInput"))
      (for _array_element _outrownames
        (bind _returnvalue (`|GetDataTableRow` "/Game/ProjectZeroAssets/Blueprints/KeyMapping/T_DefaultActionInput.T_DefaultActionInput" _array_element)
          (:`then`
            (`KismetArrayLibrary.Array_Add` _actioninputs _returnvalue)))))
    (:`then_1`
      (bind _outrownames_2 (`DataTableFunctionLibrary.GetDataTableRowNames` "/Game/ProjectZeroAssets/Blueprints/KeyMapping/T_DefaultAxisInput.T_DefaultAxisInput"))
      (for _array_element_2 _outrownames_2
        (bind _returnvalue_2 (`|GetDataTableRow` "/Game/ProjectZeroAssets/Blueprints/KeyMapping/T_DefaultAxisInput.T_DefaultAxisInput" _array_element_2)
          (:`then`
            (`KismetArrayLibrary.Array_Add` _axisinputs _returnvalue_2)))))
    (:`then_2`
      (return (`local.info`)))))

(fn `LoadMapping`
  (returns (Info :type "/Game/ProjectZeroCore/KeyRemappingSys/S_Save Structure") (`NoSave?` :type Boolean))
  (bind _returnvalue (`GameplayStatics.DoesSaveGameExist` "Player"))
  (if _returnvalue
    _
    (else
      _))
  (bind _info1 (`self.LoadDefaultMapping` null))
  (return _info1 true))

(fn `SaveMapping`
  (params (Info :type "/Game/ProjectZeroCore/KeyRemappingSys/S_Save Structure"))
  (locals (SlotName :type String :default "Player"))
  (bind _slotname (`local.SlotName`))
  (bind _returnvalue (`GameplayStatics.DoesSaveGameExist` _slotname))
  (if _returnvalue
    (bind _returnvalue_2 (`GameplayStatics.LoadGameFromSlot` _slotname))
    (bind _asbp_save (cast `/Game/ProjectZeroAssets/Blueprints/KeyMapping/BP_Save` _returnvalue_2))
    (set `/Game/ProjectZeroAssets/Blueprints/KeyMapping/BP_Save.Info` Info _asbp_save)
    (`GameplayStatics.SaveGameToSlot` _returnvalue_2 _slotname)
    (else
      (bind _returnvalue_3 (`GameplayStatics.CreateSaveGameObject` "/Game/ProjectZeroAssets/Blueprints/KeyMapping/BP_Save.BP_Save_C"))
      (set `/Game/ProjectZeroAssets/Blueprints/KeyMapping/BP_Save.Info` Info _returnvalue_3)
      (`GameplayStatics.SaveGameToSlot` _returnvalue_3 _slotname))))