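; Player controller that drives the controlled character: movement, look, jump, FPS/TPS camera switching and interaction.
; Construction loads state, inventory and HUD info from row data; BeginPlay loads key mappings, wakes the inventory and creates the HUD.
; Tick polls mapped keys into key events and diffs sync maps against current state, firing update events.
; A camera line trace focuses interaction components and forwards keys to them.
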(event `InputAxis|MoveForward` :overrideparent false
  (params (AxisValue :type "Float (single-precision)"))
  (bind _characterref (`self.CharacterRef`))
  ;[1 1 1] Base Control
  (if true
    (`/Engine/EditorBlueprintResources/StandardMacros.IsValid` _characterref
      (:`Is Valid`
        (`Pawn.AddMovementInput` _characterref (`KismetMathLibrary.GetForwardVector` (`KismetMathLibrary.MakeRotator` 0.0 0.0 (.yaw (`self.GetControlRotation`)))) AxisValue false)))))

(event `InputAxis|MoveRight` :overrideparent false
  (params (AxisValue :type "Float (single-precision)"))
  (bind _characterref (`self.CharacterRef`))
  ;[1 1 1] Base Control
  (if true
    (`/Engine/EditorBlueprintResources/StandardMacros.IsValid` _characterref
      (:`Is Valid`
        (`Pawn.AddMovementInput` _characterref (`KismetMathLibrary.GetRightVector` (`KismetMathLibrary.MakeRotator` 0.0 0.0 (.yaw (`self.GetControlRotation`)))) AxisValue false)))))

(event `InputAxis|Turn` :overrideparent false
  (params (AxisValue :type "Float (single-precision)"))
  (bind _characterref (`self.CharacterRef`))
  ;[1 1 1] Base Control
  (`/Engine/EditorBlueprintResources/StandardMacros.IsValid` _characterref
    (:`Is Valid`
      (`Pawn.AddControllerYawInput` _characterref AxisValue))))

(event `InputAxis|LookUp` :overrideparent false
  (params (AxisValue :type "Float (single-precision)"))
  (bind _characterref (`self.CharacterRef`))
  ;[1 1 1] Base Control
  (`/Engine/EditorBlueprintResources/StandardMacros.IsValid` _characterref
    (:`Is Valid`
      (`Pawn.AddControllerPitchInput` _characterref AxisValue))))

(event `self.ReceiveBeginPlay`
  ;[1 1 1] Event Begin Player
  (`self.InitPlayer`)
  (`self.BindEvent`))

(event `SwitchViewMode`
  (bind _characterref (`self.CharacterRef`))
  (bind _charactermovement (`Character.CharacterMovement` _characterref))
  (bind _followcamera (`/Game/ProjectZeroAssets/Blueprints/Players/Player_Character.FollowCamera` _characterref))
  ;[1 0.1076 0.1076] Event
  (switch `/Game/ProjectZeroCore/PlayerSys/E_PlayerEnumValue` (`BlueprintMapLibrary.Map_Find` (`.EnumMap_22_58848A47EA44FD997A48A0A3E29FBD7C` (break `/Game/ProjectZeroCore/PlayerSys/S_PlayerState` (`.State_40_F77820470D4335EAFDFEE0A8C4ED2D57` (break `/Game/ProjectZeroCore/PlayerSys/S_PlayerInfo` (`self.info`))))) "NewEnumerator1")
    (:`NewEnumerator2`
      (set `Pawn.bUseControllerRotationYaw` false _characterref)
      (set `CharacterMovementComponent.bOrientRotationToMovement` true _charactermovement)
      (set `CameraComponent.bUsePawnControlRotation` false _followcamera)
      (bind (_direction _newtrack_0) (`Timeline|Timeline_0` :!label _label)
        (:`Update`
          (set `SpringArmComponent.TargetArmLength` (`KismetMathLibrary.Lerp` 0.0 375.0 _newtrack_0) (`/Game/ProjectZeroAssets/Blueprints/Players/Player_Character.CameraBoon` _characterref)))))
    (:`NewEnumerator1`
      (set `Pawn.bUseControllerRotationYaw` true _characterref)
      (set `CharacterMovementComponent.bOrientRotationToMovement` false _charactermovement)
      (set `CameraComponent.bUsePawnControlRotation` true _followcamera)
      (goto _label :!via `Reverse`))))

(event `self.ReceiveTick`
  (params (DeltaSeconds :type "Float (single-precision)"))
  (bind _bindkeyupdate (`self.BindKeyUpdate`))
  (bind _itcomponent (`self.ITComponent`))
  (bind (_boolmap _floatmap _enummap) (break `/Game/ProjectZeroCore/PlayerSys/S_PlayerState` (`self.StateSync`)))
  (bind _boolmap_2 (break `/Game/ProjectZeroCore/UISys/S_UIState` (`.State_5_03B5C48CB6413F8D41B4B3A762333463` (break `/Game/ProjectZeroCore/UISys/S_UI` (`self.UiInfo`)))))
  (bind (_boolmap_3 _floatmap_2 _enummap_2) (break `/Game/ProjectZeroCore/PlayerSys/S_PlayerState` (`.State_40_F77820470D4335EAFDFEE0A8C4ED2D57` (break `/Game/ProjectZeroCore/PlayerSys/S_PlayerInfo` (`self.info`)))))
  ;[1 1 1] Event Tick
  (if (`self.CanTick?`)
    ;[1 1 1] Listen Key Input
    (`|ExecutionSequence`
      (:`then_0`
        (for _array_element (`.ActionInputs_3_C8F61655F34696358FA99EBD9246B3CA` (break `/Game/ProjectZeroCore/KeyRemappingSys/S_Save` (`self.SaveInfo`)))
          (bind (_keys _identifier) (break `/Game/ProjectZeroCore/KeyRemappingSys/S_ActionInput` _array_element))
          (for _array_element_2 _keys
            (if (`self.IsInputKeyDown` _array_element_2)
              (if (== (`BlueprintMapLibrary.Map_Find` _bindkeyupdate _identifier) false)
                (`BlueprintMapLibrary.Map_Add` _bindkeyupdate _identifier true)
                (`self.Key` _identifier))
              (elif (== (`BlueprintMapLibrary.Map_Find` _bindkeyupdate _identifier) true)
                (`BlueprintMapLibrary.Map_Add` _bindkeyupdate _identifier)
                (`self.Key` _identifier true))))))
      (:`then_1`
        ;[1 1 1] Compare State
        (bind (_key _value) (`/Game/ProjectZeroCore/Utils/ActorMacros.CompareBoolMap` _boolmap _boolmap_3)
          (:`Then`
            (`BlueprintMapLibrary.Map_Add` _boolmap_3 (cast `/Game/ProjectZeroCore/PlayerSys/E_PlayerBool` _key) _value))
          (:`Complete`
            (bind (_key_2 _value_2) (`/Game/ProjectZeroCore/Utils/ActorMacros.CompareFloatMap` _floatmap _floatmap_2)
              (:`Then`
                (bind _returnvalue (cast `/Game/ProjectZeroCore/PlayerSys/E_PlayerFloat` _key_2))
                (`BlueprintMapLibrary.Map_Add` _floatmap_2 _returnvalue _value_2)
                (`self.UpdateFloat` _returnvalue _value_2))
              (:`Completed`
                (bind (_key_3 _value_3) (`/Game/ProjectZeroCore/Utils/ActorMacros.CompareByteMap` _enummap _enummap_2)
                  (:`Then`
                    (bind _returnvalue_2 (cast `/Game/ProjectZeroCore/PlayerSys/E_PlayerEnumKey` _key_3))
                    (bind _returnvalue_3 (cast `/Game/ProjectZeroCore/PlayerSys/E_PlayerEnumValue` _value_3))
                    (`BlueprintMapLibrary.Map_Add` _enummap_2 _returnvalue_2 _returnvalue_3)
                    (`self.UpdateEnum` _returnvalue_2 _returnvalue_3))
                  (:`Completed`
                    (bind (_key_4 _value_4) (`/Game/ProjectZeroCore/Utils/ActorMacros.CompareBoolMap` (`.BoolMap_4_3C68399FD44BB17977E8E2AB352E0D3D` (break `/Game/ProjectZeroCore/UISys/S_UIState` (`self.UIStateSync`))) _boolmap_2)
                      (:`Then`
                        (bind _returnvalue_4 (cast `/Game/ProjectZeroCore/UISys/E_UIBool` _key_4))
                        (`BlueprintMapLibrary.Map_Add` _boolmap_2 _returnvalue_4 _value_4)
                        (`self.UpdateUIBool` _returnvalue_4 _value_4))))))))))
      (:`then_2`
        ;[1 1 1] Check Focus
        (bind _interablecomponent (`self.GetInterAbleActor`))
        (`/Engine/EditorBlueprintResources/StandardMacros.IsValid` _interablecomponent
          (:`Is Valid`
            (if (not (== _interablecomponent _itcomponent))
              (`|ExecutionSequence`
                (:`then_0`
                  (`/Engine/EditorBlueprintResources/StandardMacros.IsValid` _itcomponent :!label _label_2
                    (:`Is Valid`
                      (`/Game/ProjectZeroAssets/Blueprints/Components/Interaction/InteractionComponent.Focus` _itcomponent false)
                      (set `self.ITComponent` null))))
                (:`then_1`
                  (bind _output_get (set `self.ITComponent` _interablecomponent))
                  (`/Game/ProjectZeroAssets/Blueprints/Components/Interaction/InteractionComponent.Focus` _output_get true)))))
          (:`Is Not Valid`
            (goto _label_2)))))
    (elif (`KismetSystemLibrary.IsValid` (`self.CharacterRef`))
      (set `self.CanTick?` true))))

(event `BindEvent`
  ;[1 1 1] Bind Key Event
  (`|ExecutionSequence`
    (:`then_0`
      (add `self.Key` (delegate `Key_Event`)))
    (:`then_1`
      (add `self.UpdateFloat` (delegate `UpdateFloat_Event`))
      (add `self.UpdateEnum` (delegate `UpdateEnum_Event`)))))

(event `Key_Event` :!signature `self.Key`
  (params (Key :type "/Game/ProjectZeroCore/KeyRemappingSys/E_KeyBinding Enum") (isRelease :type Boolean))
  (bind _characterref (`self.CharacterRef`))
  (bind (_boolmap _floatmap _enummap) (break `/Game/ProjectZeroCore/PlayerSys/S_PlayerState` (`self.StateSync`)))
  (bind _boolmap_2 (break `/Game/ProjectZeroCore/UISys/S_UIState` (`self.UIStateSync`)))
  ;[1 1 1] Bind Key Event
  (`|ExecutionSequence`
    (:`then_0`
      (`self.DispatchKey` Key isRelease))
    (:`then_1`
      (switch `/Game/ProjectZeroCore/KeyRemappingSys/E_KeyBinding` Key
        (:`NewEnumerator25`
          (`/Game/ProjectZeroCore/Utils/ActorMacros.CheckInput` isRelease
            (:`Press`
              (`/Engine/EditorBlueprintResources/StandardMacros.FlipFlop`
                (:`A`
                  (`BlueprintMapLibrary.Map_Add` _enummap "NewEnumerator1" "NewEnumerator1"))
                (:`B`
                  (`BlueprintMapLibrary.Map_Add` _enummap "NewEnumerator1" "NewEnumerator2"))))))
        (:`NewEnumerator10`
          (`/Game/ProjectZeroCore/Utils/ActorMacros.CheckInput` isRelease
            (:`Press`
              (`Character.Jump` _characterref))
            (:`Release`
              (`Character.StopJumping` _characterref))))
        (:`NewEnumerator26`
          (`/Game/ProjectZeroCore/Utils/ActorMacros.CheckInput` isRelease
            (:`Press`
              (`BlueprintMapLibrary.Map_Add` _boolmap_2 "NewEnumerator1" (not (`BlueprintMapLibrary.Map_Find` _boolmap_2 "NewEnumerator1"))))))
        (:`NewEnumerator28`
          (`/Game/ProjectZeroCore/Utils/ActorMacros.CheckInput` isRelease
            (:`Press`
              (`BlueprintMapLibrary.Map_Add` _boolmap_2 "NewEnumerator2" (not (`BlueprintMapLibrary.Map_Find` _boolmap_2 "NewEnumerator2"))))))))))

(event `UpdateFloat_Event` :!signature `self.UpdateFloat`
  (params (Key :type "/Game/ProjectZeroCore/PlayerSys/E_PlayerFloat Enum") (Value :type "Float (double-precision)"))
  ;[1 1 1] Bind Key Event
  (switch `/Game/ProjectZeroCore/PlayerSys/E_PlayerFloat` Key))

(event `UpdateEnum_Event` :!signature `self.UpdateEnum`
  (params (Key :type "/Game/ProjectZeroCore/PlayerSys/E_PlayerEnumKey Enum") (Value :type "/Game/ProjectZeroCore/PlayerSys/E_PlayerEnumValue Enum"))
  ;[1 1 1] Bind Key Event
  (switch `/Game/ProjectZeroCore/PlayerSys/E_PlayerEnumKey` Key
    (:`NewEnumerator1`
      (`self.SwitchViewMode`))))

(fn `DispatchKey`
  (params (Key :type "/Game/ProjectZeroCore/KeyRemappingSys/E_KeyBinding Enum") (IsRelease :type Boolean))
  (bind _interablecomponent (`self.GetInterAbleActor`))
  (`/Engine/EditorBlueprintResources/StandardMacros.IsValid` _interablecomponent
    (:`Is Valid`
      (`/Game/ProjectZeroAssets/Blueprints/Components/Interaction/InteractionComponent.Key` _interablecomponent Key IsRelease))))

(fn `GetInterAbleActor`
  (returns (InterableComponent :type "/Game/ProjectZeroAssets/Blueprints/Components/Interaction/InteractionComponent Object Reference") (HitActor :type "Actor Object Reference"))
  (bind _characterref (`self.CharacterRef`))
  (bind _followcamera (`/Game/ProjectZeroAssets/Blueprints/Players/Player_Character.FollowCamera` _characterref))
  (bind _returnvalue (`SceneComponent.K2_GetComponentLocation` _followcamera))
  (bind _outhit (`KismetSystemLibrary.LineTraceSingleForObjects` _returnvalue (+ _returnvalue (* (`KismetMathLibrary.Conv_RotatorToVector` (`SceneComponent.K2_GetComponentRotation` _followcamera)) (+ (`SpringArmComponent.TargetArmLength` (`/Game/ProjectZeroAssets/Blueprints/Players/Player_Character.CameraBoon` _characterref)) (`BlueprintMapLibrary.Map_Find` (`.FloatMap_31_A8D7F38EC544AA2B7390548CDD99F56C` (break `/Game/ProjectZeroCore/PlayerSys/S_PlayerState` (`self.StateSync`))) "NewEnumerator4")))) (`|MakeArray` "ObjectTypeQuery1" "ObjectTypeQuery2" "ObjectTypeQuery3" :!type "EObjectTypeQuery Enum") false (`|MakeArray` _characterref :!type "Actor Object Reference")))
  (bind (_bblockinghit _binitialoverlap _time _location _impactpoint _normal _impactnormal _physmat _hitactor) (`GameplayStatics.BreakHitResult` _outhit))
  (`/Engine/EditorBlueprintResources/StandardMacros.IsValid` _hitactor
    (:`Is Valid`
      (bind _returnvalue_2 (`self.GetComponentByClass` _hitactor "/Game/ProjectZeroAssets/Blueprints/Components/Interaction/InteractionComponent.InteractionComponent_C"))
      (`/Engine/EditorBlueprintResources/StandardMacros.IsValid` _returnvalue_2
        (:`Is Valid`
          (return _returnvalue_2 _hitactor))
        (:`Is Not Valid`
          (return null _hitactor))))
    (:`Is Not Valid`
      (return null null))))

(fn `InitInventory`
  (params (InventoryCache :type "/Game/ProjectZeroCore/InventorySys/S_Inventory Structure")))

(fn `InitPlayer`
  (`|ExecutionSequence`
    (:`then_0`
      (`|ExecutionSequence`
        (:`then_0`
          (bind _info (`/Game/ProjectZeroAssets/Blueprints/KeyMapping/BPL_Save.LoadMapping`))
          (set `self.SaveInfo` _info))
        (:`then_1`
          (bind _asplayer_character (cast `/Game/ProjectZeroAssets/Blueprints/Players/Player_Character` (`self.K2_GetPawn`)))
          (bind _output_get (set `self.CharacterRef` _asplayer_character))
          (set `/Game/ProjectZeroAssets/Blueprints/Players/Player_Character.ControlRef` self _output_get))
        (:`then_2`
          (`/Game/ProjectZeroAssets/Blueprints/Inventory/InventoryManager.Awake` (`self.InventoryManagerConponent`) (`self.InventoryComponent`)))
        (:`then_3`
          (bind _returnvalue (`|CreateWidget` (`.Class_19_B6F73FCD2B41740025F15680458512E3` (break `/Game/ProjectZeroCore/UISys/S_UI` (`self.UiInfo`)))))
          (bind _aswbp_rpghud1 (cast `/Game/ProjectZeroAssets/Blueprints/Widget/WBP_RPGHUD1` _returnvalue))
          (bind _output_get_2 (set `self.MainHudRef` _aswbp_rpghud1))
          (`UserWidget.AddToViewport` _output_get_2 0))))))

(fn `UserConstructionScript`
  (bind _inventorymanagerconponent (`self.InventoryManagerConponent`))
  (bind _out_row (`/Game/ProjectZeroCore/Utils/ObjMacros.GetRow` (`.Row_4_E5DBD683244E88065D64AC9ADF831859` (break `/Game/ProjectZeroCore/PlayerSys/S_PlayerInfo` (`self.info`)))))
  (bind _output_get (set `self.info` _out_row))
  (`|ExecutionSequence`
    (:`then_0`
      (bind ((`Inventory_37_87ACEC7244440303FD6DDFA9E26FE72B` _inventory) (`MainHud_46_7AE750DB344444726957EBB55D1AAF77` _mainhud) (`CurrentState_29_6D7A9917A5499402B000348CF7C45ACB` _currentstate) (`StateMap_34_059AB71C244538AC3B4FA98B969DFED5` _statemap)) (break `/Game/ProjectZeroCore/PlayerSys/S_PlayerInfo` _output_get))
      (bind _output_get_2 (set `self.StateMap` _statemap))
      (bind _output_get_3 (set `self.CurrentState` _currentstate))
      (set `self.StateSync` (`BlueprintMapLibrary.Map_Find` _output_get_2 _output_get_3)))
    (:`then_1`
      (bind _out_row_2 (`/Game/ProjectZeroCore/Utils/ObjMacros.GetRow` _inventory))
      (bind ((`Inventory_19_66B9714575435BAB8B1C5996A937B12B` _inventory_2) (`Currency_28_A7D9E5D7CD4680AA0017D29509FD926B` _currency)) (break `/Game/ProjectZeroCore/InventorySys/S_Inventory` _out_row_2))
      (for _array_element _inventory_2
        (bind (_row _intmap) (break `/Game/ProjectZeroCore/InventorySys/S_InventoryItem` _array_element))
        (bind (_out_row_3 _returnvalue) (`/Game/ProjectZeroCore/Utils/ObjMacros.GetRow` _row))
        (`|ExecutionSequence`
          (:`then_0`
            (`/Game/ProjectZeroCore/Utils/ObjMacros.SyncIntMap` _intmap (`.IntMap_16_5E024D6D524B4D6202191CB6B82F4C76` (break `/Game/ProjectZeroCore/InventorySys/S_ItemState` (`.State_73_4D649F467E4716F315B4B6B9EC505930` (break `/Game/ProjectZeroCore/InventorySys/S_Item` _out_row_3))))))
          (:`then_1`
            (set `/Game/ProjectZeroAssets/Blueprints/Inventory/InventoryManager.CurrencyMap` _currency _inventorymanagerconponent))
          (:`then_2`
            (`BlueprintMapLibrary.Map_Add` (`/Game/ProjectZeroAssets/Blueprints/Inventory/InventoryManager.InventoryCache` _inventorymanagerconponent) _returnvalue _out_row_3)))))
    (:`then_2`
      (bind _out_row_4 (`/Game/ProjectZeroCore/Utils/ObjMacros.GetRow` _mainhud))
      (bind _output_get_4 (set `self.UiInfo` _out_row_4))
      (`|ExecutionSequence`
        (:`then_0`
          (bind ((`CurrentState_14_7C72A78B23414C68DF9507850E4FD714` _currentstate_2) (`StateMap_13_B1E2DEB1354C015E66EFCFAE92365E65` _statemap_2)) (break `/Game/ProjectZeroCore/UISys/S_UI` _output_get_4))
          (bind _output_get_5 (set `self.CurrentUIState` _currentstate_2))
          (bind _output_get_6 (set `self.UIStateMap` _statemap_2))
          (set `self.UIStateSync` (`BlueprintMapLibrary.Map_Find` _output_get_6 _output_get_5)))))))