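; Player character Blueprint built from modular skeletal meshes for the head, main hand and off hand.
; Each OnChange function applies its part's mesh variable with a pose reinit, then sets the body Mesh as master pose component so the part follows its animation.
; The OnCommands and OnKey input hooks are stubs that return false, and the construction script is empty.
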(fn `OnChange_Head`
  (`SkinnedMeshComponent.SetSkinnedAssetAndUpdate` (`self.Head`) (`self.HeadMesh`) true)
  (`SkinnedMeshComponent.SetLeaderPoseComponent` (`self.Head`) (`self.Mesh`)))

(fn `OnChange_MainHand`
  (bind _mainhand (`self.MainHand`))
  (`SkinnedMeshComponent.SetSkinnedAssetAndUpdate` _mainhand (`self.MainHandMesh`) true)
  (`SkinnedMeshComponent.SetLeaderPoseComponent` _mainhand (`self.Mesh`)))

(fn `OnChange_OffHand`
  (bind _offhand (`self.OffHand`))
  (`SkinnedMeshComponent.SetSkinnedAssetAndUpdate` _offhand (`self.OffHandMesh`) true)
  (`SkinnedMeshComponent.SetLeaderPoseComponent` _offhand (`self.Mesh`)))

(fn `OnCommands`
  (params (CommandMap :type "Map of /Game/ProjectZeroCore/Utils/E_Operator Enum to /Game/ProjectZeroCore/Utils/S_Parse Structure"))
  (returns (NewParam :type Boolean))
  (return false))

(fn `OnKey`
  (params (Key :type "/Game/ProjectZeroCore/KeyRemappingSys/E_KeyBinding Enum" :default "NewEnumerator0") (Value :type Boolean))
  (returns (NewParam :type Boolean))
  (return false))

(fn `UserConstructionScript`)